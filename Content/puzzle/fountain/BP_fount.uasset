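; Puzzle fountain that reveals its water meshes and a key actor when three vent states match a set combination.
; CheckVents tests the vent booleans and calls ActivateFountain, which unhides Cylinder, Fountain and Key1 and plays a water sound.
; DisactivateFountain hides the root and Fountain components and stops audio.
; The vent-setting chains in the EventGraph are disconnected, and nothing here calls DisactivateFountain.
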(event `self.fountain.OnComponentBeginOverlap`
  (params (OverlappedComponent :type "PrimitiveComponent Object Reference") (OtherActor :type "Actor Object Reference") (OtherComp :type "PrimitiveComponent Object Reference") (OtherBodyIndex :type Integer) (bFromSweep :type Boolean) (SweepResult :type "HitResult Structure (by ref)")))

(event `self.ReceiveBeginPlay`
  (set `self.water_ref` (`self.Cylinder`)))

(event `self.uploads_files_5495422_Fountain_4.OnComponentEndOverlap`
  (params (OverlappedComponent :type "PrimitiveComponent Object Reference") (OtherActor :type "Actor Object Reference") (OtherComp :type "PrimitiveComponent Object Reference") (OtherBodyIndex :type Integer)))

(fn `ActivateFountain`
  (locals (NewLocalVar :type "Vector Structure" :default (0.0 0.0 0.0)))
  (`SceneComponent.SetVisibility` (`self.Cylinder`) true false)
  (`SceneComponent.SetVisibility` (`self.fountain`) true false)
  (`self.SetActorHiddenInGame` (`self.key1`) false)
  (if (`KismetSystemLibrary.IsValid` (`self.Audio1`))
    (`GameplayStatics.PlaySoundAtLocation` "/Game/fountain/Download_Water_Liquid_Large_Fountain_Sm_B01_Sound_Effect_Royalty.Download_Water_Liquid_Large_Fountain_Sm_B01_Sound_Effect_Royalty" (`self.K2_GetActorLocation` (`ActorComponent.GetOwner` (`self.fountain`))) (struct) 1.0 1.0 0.0 null null null null)))

(fn `CheckVents`
  (if (and (== (`self.vent1State`) true) (== (`self.vent2State`) false) (== (`self.vent3State`) true))
    (`self.ActivateFountain`)))

(fn `Disactivate Fountain`
  (bind _audio (`self.audio`))
  (`SceneComponent.SetVisibility` (`self.RootComponent`) false false)
  (`SceneComponent.SetVisibility` (`self.fountain`) false false)
  (if (`KismetSystemLibrary.IsValid` _audio)
    (`AudioComponent.Stop` _audio)))

(fn `UserConstructionScript`)