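; BP_puzzle is a collect-items puzzle actor that reveals a portal once enough items are gathered.
; It plays a 2D music cue on BeginPlay and counts pickups through the collectitem event.
; When the count reaches the maximum, a DoOnce gate calls VisibleTeleport, which makes the Niagara GPU portal effect visible.
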(event `self.ReceiveBeginPlay`
  (`GameplayStatics.PlaySound2D` "/Game/puzzle/collect_items/StockTune-Surreal_Sonic_Voyage_1741489402_Cue.StockTune-Surreal_Sonic_Voyage_1741489402_Cue" 1.0 1.0 0.0 null null))

(event `collect item`
  (`/Engine/EditorBlueprintResources/StandardMacros.IncrementInt` (`self.currentCollect_Items`)
    (:`  `
      (if (>= (`self.currentCollect_Items`) (`self.maxCollect_Items`))
        (`/Engine/EditorBlueprintResources/StandardMacros.DoOnce` false
          (:`Completed`
            (`self.visible teleport`)))))))

(event `visible teleport`
  (`SceneComponent.SetVisibility` (`self.NS_GpuPortal`) true false))

(fn `UserConstructionScript`)